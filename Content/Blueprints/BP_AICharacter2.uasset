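; BP_AICharacter2 is an AI character Blueprint that visualizes its PawnSensing sight range for debugging.
; Every tick it draws a red debug cone from the capsule along the actor's forward vector, sized by the sensing component's sight radius and peripheral vision angle.
; It also prints the sine of that angle each tick.
; No sensing response or other behavior is implemented in its graphs.
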(event EventBeginPlay)

(event Collision|EventActorBeginOverlap
  (params (OtherActor :type Actor%20Object%20Reference)))

(event EventTick
  (params (DeltaSeconds :type Float%20%28single-precision%29))
  (bind _pawnsensingcomp (Variables|Default|GetPawnSensingComp))
  (bind _peripheralvisionangle (Variables|/Script/AIModule.PawnSensingComponent|GetPeripheralVisionAngle _pawnsensingcomp))
  (Class|KismetSystemLibrary|DrawDebugConeinDegrees (Transformation|GetWorldLocation (Variables|Default|GetCapsuleComponent)) (Math|Vector|GetForwardVector (Transformation|GetActorRotation)) (Variables|/Script/AIModule.PawnSensingComponent|GetSightRadius _pawnsensingcomp) _peripheralvisionangle _peripheralvisionangle 12 "(R=0.970000,G=0.053350,B=0.053350,A=1.000000)" 0.0 5.0)
  (Development|PrintString (Utilities|String|ToString(Float) (Math|Trig|Sin(Degrees) _peripheralvisionangle))))

(fn ConstructionScript)